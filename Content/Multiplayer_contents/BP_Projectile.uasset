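; Multiplayer projectile that damages a BP_MultiplayerPawn on overlap and shows an explosion.
; The server moves it forward each Tick by Speed without sweep, and a TTL timer triggers its delayed destruction.
; Sphere overlaps run a server collision check that compares against the owner, applies Damage, multicasts the explosion emitter and destroys the actor after a short delay.
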(event `self.ReceiveBeginPlay`
  ;[1 1 1] уничтожение снаряда по таймеру
  (`KismetSystemLibrary.K2_SetTimerDelegate` (delegate `LifeEnabled`) (`self.TTL`)))

(event `Server_LifeEnabled`
  ;[1 1 1] уничтожение снаряда по таймеру
  (`KismetSystemLibrary.Delay` 0.2)
  (`self.K2_DestroyActor`))

(event `LifeEnabled`
  ;[1 1 1] уничтожение снаряда по таймеру
  (`self.Server_LifeEnabled`))

(event `Server_Move`
  (params (DeltaTime :type "Float (double-precision)"))
  ;[1 1 1] передвижение снаряда
  (`self.K2_SetActorLocation` (+ (`self.K2_GetActorLocation`) (* (`self.GetActorForwardVector`) (* DeltaTime (`self.Speed`))))))

(event `self.ReceiveTick`
  (params (DeltaSeconds :type "Float (single-precision)"))
  ;[1 1 1] полёт снаряда на сервере
  (if (`KismetSystemLibrary.IsServer`)
    (`self.Server_Move` DeltaSeconds)))

(event `Server_Collision`
  (params (OtherActor :type "Actor Object Reference") (Location :type "Vector Structure"))
  ;[1 1 1] события при коллизии с чем-либо
  (if (!= OtherActor (`self.GetOwner`))
    (bind _asbp_multiplayer_pawn (cast `/Game/Multiplayer_contents/BP_MultiplayerPawn` OtherActor))
    (`/Game/Multiplayer_contents/BP_MultiplayerPawn.Take_Damage` _asbp_multiplayer_pawn (`self.Damage`))
    (else
      (cast `/Game/Multiplayer_contents/BP_Projectile` OtherActor
        (:`CastFailed`
          _))))
  (`self.Multicast_HitEffects` Location)
  (`self.Server_LifeEnabled`))

(event `self.Sphere.OnComponentBeginOverlap`
  (params (OverlappedComponent :type "PrimitiveComponent Object Reference") (OtherActor :type "Actor Object Reference") (OtherComp :type "PrimitiveComponent Object Reference") (OtherBodyIndex :type Integer) (bFromSweep :type Boolean) (SweepResult :type "HitResult Structure (by ref)"))
  ;[1 1 1] при коллизии запустить проверку коллизии
  (if (`KismetSystemLibrary.IsServer`)
    (`self.Server_Collision` OtherActor (`self.K2_GetActorLocation`))))

(event `SpawnHitEffects`
  (params (HitLocation :type "Vector Structure"))
  ;[1 1 1] событие взрыва
  (`GameplayStatics.SpawnEmitterAtLocation` "/Game/StarterContent/Particles/P_Explosion.P_Explosion" HitLocation))

(event `Multicast_HitEffects`
  (params (HitLocation :type "Vector Structure"))
  ;[1 1 1] мультикаст функция вызова взрыва
  (`self.SpawnHitEffects` HitLocation))

(fn `UserConstructionScript`)