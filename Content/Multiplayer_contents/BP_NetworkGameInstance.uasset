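; Game instance that hosts, lists and joins LAN multiplayer sessions.
; CreateGame creates a four-slot session and opens Level1 as a listen server.
; GetGames fills a Sessions map keyed by server name, player count and ping text, exposed through GetSessions.
; JoinToGame joins the single result of its own search, and failures, including network and travel errors, are printed to screen.
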(event `CreateGame`
  ;[1 1 1] создание игры
  (`CreateSessionCallbackProxy.CreateSession` (`GameplayStatics.GetPlayerController` 0) 4 true
    (:`OnSuccess`
      (`GameplayStatics.OpenLevel` "Level1" true "listen"))
    (:`OnFailure`
      (`KismetSystemLibrary.PrintString` "Game creation error!"))))

(event `GetGames`
  (bind _sessions (`self.Sessions`))
  ;[1 1 1] получение информации о серверах
  (`BlueprintMapLibrary.Map_Clear` (`self.Sessions`))
  (bind _results (`FindSessionsCallbackProxy.FindSessions` (`GameplayStatics.GetPlayerController` 0) 4 true)
    (:`OnSuccess`
      (for _array_element _results
        (`BlueprintMapLibrary.Map_Add` _sessions (`KismetStringLibrary.Concat_StrStr` "Server: " (`FindSessionsCallbackProxy.GetServerName` _array_element) " Players: " (`KismetStringLibrary.Conv_IntToString` (`FindSessionsCallbackProxy.GetCurrentPlayers` _array_element)) "/" (`KismetStringLibrary.Conv_IntToString` (`FindSessionsCallbackProxy.GetMaxPlayers` _array_element)) " Ping:" (`KismetStringLibrary.Conv_IntToString` (`FindSessionsCallbackProxy.GetPingInMs` _array_element))) _array_element)
        (if (> (`BlueprintMapLibrary.Map_Length` _sessions) 0)
          (`KismetSystemLibrary.PrintString` "Sessions added" true true (struct :`G` 0.66 :`B` 1.0 :`A` 1.0) 10.0)
          (else
            (`KismetSystemLibrary.PrintString` "array 1 error" true true (struct :`G` 0.66 :`B` 1.0 :`A` 1.0) 10.0)))))
    (:`OnFailure`
      (`KismetSystemLibrary.PrintString` "Game find error!" true true (struct :`G` 0.66 :`B` 1.0 :`A` 1.0) 10.0))))

(event `JoinToGame`
  (bind _returnvalue (`GameplayStatics.GetPlayerController` 0))
  ;[1 1 1] подключение к рандомной сессии
  (bind _results (`FindSessionsCallbackProxy.FindSessions` _returnvalue 1 true)
    (:`OnSuccess`
      (for _array_element _results
        (`JoinSessionCallbackProxy.JoinSession` _returnvalue _array_element
          (:`OnFailure`
            (`KismetSystemLibrary.PrintString` "Join to game error!")))))
    (:`OnFailure`
      (`KismetSystemLibrary.PrintString` "Game searching error!"))))

(event `self.HandleNetworkError`
  (params (FailureType :type "ENetworkFailure Enum" :default "NetDriverAlreadyExists") (bIsServer :type Boolean))
  ;[1 1 1] обработка ошибок сервера
  (`KismetSystemLibrary.PrintString` (`KismetStringLibrary.Concat_StrStr` "Network error: " (`|GetEnumeratorNameAsString` FailureType) " on server?" (`KismetStringLibrary.Conv_BoolToString` bIsServer)) true true (struct :`G` 0.66 :`B` 1.0 :`A` 1.0) 10.0))

(event `self.HandleTravelError`
  (params (FailureType :type "ETravelFailure Enum" :default "NoLevel"))
  ;[1 1 1] обработка ошибок сервера
  (`KismetSystemLibrary.PrintString` (`KismetStringLibrary.Concat_StrStr` "Network travel error: " (`|GetEnumeratorNameAsString` FailureType))))

(fn `GetSessions`
  (returns (Sessions :type "Map of String to BlueprintSessionResult Structure"))
  (return (`self.Sessions`)))